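; Missile projectile Blueprint for an FPS weapon that produces explosion effects on overlap or when damaged.
; Actor overlap only spawns the explosion emitter; its direct-damage and creator-check nodes are disconnected.
; Any damage triggers a one-time blast guarded by an Exploded flag, applying full radial damage credited to the instigator and spawning the emitter.
; The Explode function is an empty stub, and no graph destroys the actor.
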(event `self.ReceiveActorBeginOverlap`
  (params (OtherActor :type "Actor Object Reference"))
  (`GameplayStatics.SpawnEmitterAtLocation` "/Game/FPS/Effects/WeaponEffects/Explosion/P_Explosion.P_Explosion" (`self.K2_GetActorLocation` self)))

(event `self.ReceiveAnyDamage`
  (params (Damage :type "Float (single-precision)") (DamageType :type "DamageType Object Reference") (InstigatedBy :type "Controller Object Reference") (DamageCauser :type "Actor Object Reference"))
  (if (not (`self.bExploded`))
    (set `self.bExploded` true)
    (`GameplayStatics.ApplyRadialDamage` :`BaseDamage` 100.0 :`Origin` (`self.K2_GetActorLocation` self) :`DamageRadius` 500.0 :`DamageTypeClass` "/Game/FPS/Blueprints/Weapons/DamageTypes/DT_Grenade.DT_Grenade_C" :`DamageCauser` self :`InstigatedByController` (`self.GetInstigatorController`) :`bDoFullDamage` true)
    (`GameplayStatics.SpawnEmitterAtLocation` "/Game/FPS/Effects/WeaponEffects/Explosion/P_Explosion.P_Explosion" (`self.K2_GetActorLocation` self))))

(fn `Explode`)

(fn `UserConstructionScript`)