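; Skill1 is a timed barrier skill actor that absorbs opposing bullets and destroys itself when its duration ends or its hitpoints drop below zero.
; Bullet and barrier tags pair Skill1B against BP_BulletA and Skill1A against BP_BulletB, subtracting each bullet's damage and destroying it.
; Each absorbed hit adds to an Energy total, passed as ultimate energy to player 0's BP_AssaultClass_A pawn, whichever barrier tag applies.
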(event `self.ReceiveBeginPlay`
  (`KismetSystemLibrary.Delay` (`self.Duration`))
  (`self.K2_DestroyActor`))

(event `Bullet Contact`
  (params (Sender :type "Actor Object Reference"))
  (bind _returnvalue (+ (`self.AddedEnergy`) (`self.Energy`)))
  (if (`self.ActorHasTag` Sender "BulletA")
    (if (`self.ActorHasTag` self "Skill1B")
      (bind _asbp_bullet_a (cast `/Game/FPS/Blueprints/Misc/Bullets/BP_BulletA` Sender))
      (bind _output_get (set `self.Barrier Hitpoint` (- (`self.Barrier Hitpoint`) (`/Game/FPS/Blueprints/Misc/Bullets/BP_BulletA.Damage` _asbp_bullet_a))))
      (bind _output_get_2 (set `self.Energy` _returnvalue))
      (bind _asbp_assault_class_a (cast `/Game/FPS/Blueprints/CharacterAndClasses/BP_AssaultClass_A` (`GameplayStatics.GetPlayerPawn` 0)))
      (`/Game/FPS/Blueprints/CharacterAndClasses/BP_AssaultClass_A.Set Ultimate Energy` _asbp_assault_class_a _output_get_2)
      (`self.K2_DestroyActor` Sender)
      (if (< _output_get 0.0)
        (`self.K2_DestroyActor` :!label _label)))
    (elif (`self.ActorHasTag` self "Skill1A")
      (bind _asbp_bullet_b (cast `/Game/FPS/Blueprints/Misc/Bullets/BP_BulletB` Sender))
      (bind _output_get_3 (set `self.Barrier Hitpoint` (- (`self.Barrier Hitpoint`) (`/Game/FPS/Blueprints/Misc/Bullets/BP_BulletA.Damage` _asbp_bullet_b))))
      (bind _output_get_4 (set `self.Energy` _returnvalue))
      (bind _asbp_assault_class_a_2 (cast `/Game/FPS/Blueprints/CharacterAndClasses/BP_AssaultClass_A` (`GameplayStatics.GetPlayerPawn` 0)))
      (`/Game/FPS/Blueprints/CharacterAndClasses/BP_AssaultClass_A.Set Ultimate Energy` _asbp_assault_class_a_2 _output_get_4)
      (`self.K2_DestroyActor` Sender)
      (if (< _output_get_3 0.0)
        (goto _label)))))

(fn `UserConstructionScript`)