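; Skill 2 is a team-tagged drone projectile that slows and damages opposing characters entering its detection sphere.
; It launches with a scaled shield, then zeroes MaxSpeed after VisionDuration; overlaps also swap victims' body materials and decrement charges per material slot.
; A Delay-gated Tick countdown limits its lifetime, and opposing bullets drain its hitpoints until destruction.
; Team checks use Skill2A/2B tags, except the BulletB branch, which checks Skill1B.
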(event `self.ReceiveBeginPlay`
  (bind _projectilemovement (`self.ProjectileMovement`))
  (if (> (`self.Number of Charges`) 0)
    (`SceneComponent.SetWorldScale3D` (`self.ShieldModel`) (`KismetMathLibrary.Conv_DoubleToVector` (`self.Detection Area`)))
    (set `ProjectileMovementComponent.InitialSpeed` (`self.Projectile Speed`) _projectilemovement)
    (`KismetSystemLibrary.Delay` (`self.Vision Duration`))
    (set `ProjectileMovementComponent.MaxSpeed` 0.0 _projectilemovement)
    (else
      (`self.K2_DestroyActor`))))

(event `self.Sphere.OnComponentBeginOverlap`
  (params (OverlappedComponent :type "PrimitiveComponent Object Reference") (OtherActor :type "Actor Object Reference") (OtherComp :type "PrimitiveComponent Object Reference") (OtherBodyIndex :type Integer) (bFromSweep :type Boolean) (SweepResult :type "HitResult Structure (by ref)"))
  (bind _pulse_damage (`self.Pulse Damage`))
  (bind _asbp_base_character (cast `/Game/FPS/Blueprints/CharacterAndClasses/BP_BaseCharacter` OtherActor))
  (if (`self.ActorHasTag` _asbp_base_character "TeamA")
    (if (`self.ActorHasTag` self "Skill2B")
      (`/Game/FPS/Blueprints/CharacterAndClasses/BP_BaseCharacter.SlowSpeed` _asbp_base_character (`self.Slow Amount`) (`self.SlowDuration`))
      (`GameplayStatics.ApplyDamage` OtherActor (`KismetMathLibrary.Conv_IntToDouble` _pulse_damage) null null "/Game/FPS/Blueprints/Weapons/DamageTypes/DT_AssaultRifle.DT_AssaultRifle_C")
      (bind _meshfp (`/Game/FPS/Blueprints/CharacterAndClasses/BP_BaseCharacter.MeshFP` _asbp_base_character))
      (for _index (range (`PrimitiveComponent.GetNumMaterials` _meshfp)) :!label _label
        (`PrimitiveComponent.SetMaterial` _meshfp _index "/Game/FPS/Blueprints/Skills/M_UE4Man_Body_Inst.M_UE4Man_Body_Inst")
        (`PrimitiveComponent.SetMaterial` (`Character.Mesh` _asbp_base_character) _index "/Game/FPS/Blueprints/Skills/M_UE4Man_Body_Inst.M_UE4Man_Body_Inst")
        (set `self.Number of Charges` (- (`self.Number of Charges`) 1))))
    (elif (`self.ActorHasTag` self "Skill2A")
      (`/Game/FPS/Blueprints/CharacterAndClasses/BP_BaseCharacter.SlowSpeed` _asbp_base_character (`self.Slow Amount`) (`self.SlowDuration`))
      (`GameplayStatics.ApplyDamage` OtherActor (`KismetMathLibrary.Conv_IntToDouble` _pulse_damage))
      (goto _label))))

(event `self.ReceiveTick`
  (params (DeltaSeconds :type "Float (single-precision)"))
  (if (> (`self.DroneLifeTime`) 0.0)
    (`KismetSystemLibrary.Delay` 1.0)
    (set `self.DroneLifeTime` (- (`self.DroneLifeTime`) 1.0))
    (else
      (`self.K2_DestroyActor`))))

(event `BulletCntact`
  (params (Sender :type "Actor Object Reference"))
  (if (`self.ActorHasTag` Sender "BulletA")
    (if (`self.ActorHasTag` self "Skill2B")
      (bind _asbp_bullet_a (cast `/Game/FPS/Blueprints/Misc/Bullets/BP_BulletA` Sender))
      (bind _returnvalue (- (`KismetMathLibrary.Conv_IntToDouble` (`self.Drone Hitpoint`)) (`/Game/FPS/Blueprints/Misc/Bullets/BP_BulletA.Damage` _asbp_bullet_a)))
      (set `self.Drone Hitpoint` (`KismetMathLibrary.FTrunc` _returnvalue))
      (if (< _returnvalue 0.0)
        (`self.K2_DestroyActor`)))
    (elif (`self.ActorHasTag` self "Skill1B")
      (bind _asbp_bullet_b (cast `/Game/FPS/Blueprints/Misc/Bullets/BP_BulletB` Sender))
      (bind _returnvalue_2 (- (`KismetMathLibrary.Conv_IntToDouble` (`self.Drone Hitpoint`)) (`/Game/FPS/Blueprints/Misc/Bullets/BP_BulletA.Damage` _asbp_bullet_b)))
      (set `self.Drone Hitpoint` (`KismetMathLibrary.FTrunc` _returnvalue_2))
      (if (< _returnvalue_2 0.0)
        (`self.K2_DestroyActor`)))))

(fn `ApplySelectedPerk`)

(fn `MeleeAttack`)

(fn `SetAttacking`
  (params (bool1 :type Boolean)))

(fn `UpdateAll tags`)

(fn `UserConstructionScript`)