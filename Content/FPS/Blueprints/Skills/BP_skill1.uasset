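; BP_skill1 is a timed skill area actor that calls UPdateSpeed on characters sharing its owner's team when they overlap its sphere.
; On BeginPlay it picks a mesh material by whether the owner is on player 0's team, scales by Size, and enables sphere overlaps.
; A timer destroys it after SpawnDuration.
; An ApplyDamage node exists but never runs.
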(event `self.ReceiveBeginPlay`
  (bind _staticmesh (`self.StaticMesh`))
  (`KismetSystemLibrary.Delay` 0.0)
  (if (== (`/Game/FPS/Blueprints/CharacterAndClasses/BP_BaseCharacter.bPawnTeam` (cast `/Game/FPS/Blueprints/CharacterAndClasses/BP_BaseCharacter` (`self.GetOwner`) :!pure true)) (`/Game/FPS/Blueprints/CharacterAndClasses/BP_BaseCharacter.bPawnTeam` (cast `/Game/FPS/Blueprints/CharacterAndClasses/BP_BaseCharacter` (`GameplayStatics.GetPlayerCharacter` 0) :!pure true)))
    (`PrimitiveComponent.SetMaterial` _staticmesh 0 "/Game/FPS/Blueprints/Skills/teama.teama")
    (else
      (`PrimitiveComponent.SetMaterial` _staticmesh 0 "/Game/FPS/Blueprints/Skills/teamab.teamab")))
  (`KismetSystemLibrary.K2_SetTimerDelegate` (delegate `Destroy actor`) (`self.Spawn duration`))
  (`self.SetActorScale3D` (`KismetMathLibrary.Conv_DoubleToVector` (`self.Size`)))
  (set `PrimitiveComponent.bGenerateOverlapEvents` true (`self.Sphere`)))

(event `Destroy actor`
  (`self.K2_DestroyActor`))

(event `self.Sphere.OnComponentBeginOverlap`
  (params (OverlappedComponent :type "PrimitiveComponent Object Reference") (OtherActor :type "Actor Object Reference") (OtherComp :type "PrimitiveComponent Object Reference") (OtherBodyIndex :type Integer) (bFromSweep :type Boolean) (SweepResult :type "HitResult Structure (by ref)"))
  (bind _asbp_base_character (cast `/Game/FPS/Blueprints/CharacterAndClasses/BP_BaseCharacter` OtherActor))
  (set `self.Overlapped_character` _asbp_base_character)
  (if (== (`/Game/FPS/Blueprints/CharacterAndClasses/BP_BaseCharacter.bPawnTeam` (`self.Overlapped_character`)) (`/Game/FPS/Blueprints/CharacterAndClasses/BP_BaseCharacter.bPawnTeam` (cast `/Game/FPS/Blueprints/CharacterAndClasses/BP_BaseCharacter` (`self.GetOwner`) :!pure true)))
    (`/Game/FPS/Blueprints/CharacterAndClasses/BP_BaseCharacter.UPdate_speed_` (`self.Overlapped_character`))))

(fn `UserConstructionScript`)