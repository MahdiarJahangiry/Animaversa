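; Skill3 is a team-aware projectile that explodes shortly after an enemy enters its detection zone.
; BeginPlay applies configurable body size, detection sphere size and initial speed, while a Tick-driven Delay halts movement after Duration without destroying it.
; Detection overlaps wait a delay, then use actor tags (Skill3A targets TeamB, otherwise TeamA) to damage only the overlapping actor, spawn explosion particles and destroy the projectile.
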(event `self.ReceiveBeginPlay`
  (`SceneComponent.SetWorldScale3D` (`self.Sphere`) (`KismetMathLibrary.Conv_DoubleToVector` (`self.Projectile Size`)))
  (`SceneComponent.SetWorldScale3D` (`self.Sphere1`) (`KismetMathLibrary.Conv_DoubleToVector` (`self.Detection zone Size`)))
  (set `ProjectileMovementComponent.InitialSpeed` (`KismetMathLibrary.Conv_IntToDouble` (`self.Projectile Speed`)) (`self.ProjectileMovement`)))

(event `self.Sphere1.OnComponentBeginOverlap`
  (params (OverlappedComponent :type "PrimitiveComponent Object Reference") (OtherActor :type "Actor Object Reference") (OtherComp :type "PrimitiveComponent Object Reference") (OtherBodyIndex :type Integer) (bFromSweep :type Boolean) (SweepResult :type "HitResult Structure (by ref)"))
  (`KismetSystemLibrary.Delay` (`KismetMathLibrary.Conv_IntToDouble` (`self.Delay to Explode`)))
  (if (`self.ActorHasTag` self "Skill3A")
    (if (`self.ActorHasTag` OtherActor "TeamB")
      (`GameplayStatics.ApplyDamage` OtherActor (`self.Explosion Damage`) null self "/Game/FPS/Blueprints/Weapons/DamageTypes/DT_AssaultRifle.DT_AssaultRifle_C" :!label _label)
      (`ProjectileMovementComponent.StopSimulating` (`self.ProjectileMovement`) (`GameplayStatics.MakeHitResult` false false 0.0 0.0 (0.0 0.0 0.0) (0.0 0.0 0.0) (0.0 0.0 1.0) (0.0 0.0 1.0) null self))
      (`GameplayStatics.SpawnEmitterAtLocation` "/Game/FPS/Effects/WeaponEffects/Explosion/P_Explosion.P_Explosion" (`SceneComponent.K2_GetComponentLocation` (`self.Sphere`)))
      (`self.K2_DestroyActor`))
    (elif (`self.ActorHasTag` OtherActor "TeamA")
      (goto _label))))

(event `self.ReceiveTick`
  (params (DeltaSeconds :type "Float (single-precision)"))
  (`KismetSystemLibrary.Delay` (`self.Duration`))
  (`ProjectileMovementComponent.StopSimulating` (`self.ProjectileMovement`) (`GameplayStatics.MakeHitResult` false false 0.0 0.0 (0.0 0.0 0.0) (0.0 0.0 0.0) (0.0 0.0 1.0) (0.0 0.0 1.0) null self)))

(fn `UserConstructionScript`)