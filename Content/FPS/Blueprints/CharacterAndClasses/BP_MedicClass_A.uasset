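; Medic character class for an FPS, whose first class skill spawns a medic bot.
; UseClassSkill1 spawns BP_MedicBot 1000 units above the character, assigning it the team from player controller 0 and this pawn as owner.
; AbilityCoolDown sets both the bot's lifespan and the timer that re-enables the skill.
; The gameplay widget receives that timer on use and is reset when it fires.
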(event `self.ReceiveBeginPlay`
  (`parent.ReceiveBeginPlay`))

(event `self.ReceiveTick`
  (params (DeltaSeconds :type "Float (single-precision)"))
  (`parent.ReceiveTick` DeltaSeconds))

(event `ResetSkill`
  ;[1 1 1] Reset Skill
  (set `self.bCanUseSkill1` true)
  (`/Game/FPS/WidgetBP/WB_Gameplay.Skill1Reset` (`/Game/FPS/Blueprints/PlayerController/BaseCharacterPC.GameplayWB` (cast `/Game/FPS/Blueprints/PlayerController/BaseCharacterPC` (`GameplayStatics.GetPlayerController` 0) :!pure true))))

(event `self.UseClassSkill1`
  (bind _asbase_character_pc (cast `/Game/FPS/Blueprints/PlayerController/BaseCharacterPC` (`GameplayStatics.GetPlayerController` 0) :!pure true))
  ;[1 1 1] Medic Skill
  (if (`self.bCanUseSkill1`)
    (set `self.bCanUseSkill1` false)
    (`self.SpawnMedicBot` self (`/Game/FPS/Blueprints/PlayerController/BaseCharacterPC.Team` _asbase_character_pc))
    (`GameplayStatics.PlaySound2D` "/Engine/VREditor/Sounds/UI/Invalid_Action.Invalid_Action" 1.0 1.0 0.0 null null)
    (bind _returnvalue (`KismetSystemLibrary.K2_SetTimerDelegate` (delegate `ResetSkill`) (`self.AbilityCoolDown`)))
    (`/Game/FPS/WidgetBP/WB_Gameplay.OnSkill1Used` (`/Game/FPS/Blueprints/PlayerController/BaseCharacterPC.GameplayWB` _asbase_character_pc) _returnvalue)))

(event `SpawnMedicBot`
  (params (Pawn :type "/Game/FPS/Blueprints/CharacterAndClasses/BP_BaseCharacter Object Reference") (bTeam :type Boolean))
  (bind (_returnvalue_x _returnvalue_y _returnvalue_z) (`KismetMathLibrary.BreakVector` (`self.K2_GetActorLocation` self)))
  ;[1 1 1] Spawn Medic Bot
  (bind _returnvalue (`|SpawnActorFromClass` "/Game/FPS/Blueprints/AI_Pawns/MedicBot/BP_MedicBot.BP_MedicBot_C" (`KismetMathLibrary.MakeTransform` (`KismetMathLibrary.MakeVector` _returnvalue_x _returnvalue_y (+ _returnvalue_z 1000.0)) (`self.K2_GetActorRotation` self)) "Undefined" "OverrideRootScale" Pawn (`self.AbilityCoolDown`) Pawn))
  (set `/Game/FPS/Blueprints/AI_Pawns/MedicBot/BP_MedicBot.bBotTeam` bTeam _returnvalue)
  (set `/Game/FPS/Blueprints/AI_Pawns/MedicBot/BP_MedicBot.OwnerPawn` self _returnvalue))

(fn `UserConstructionScript`
  (`parent.UserConstructionScript`))