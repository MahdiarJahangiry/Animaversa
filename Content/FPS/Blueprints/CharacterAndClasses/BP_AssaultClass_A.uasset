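; Assault class character with a timed sprint boost and three team-specific spawnable skills.
; UseClassSkill1 temporarily raises run speed through server-named events, with a timer cooldown reported to the gameplay HUD.
; Q (ground shield), F and R spawn skill actors at the character, picking the class by TeamA tag.
; R costs ultimate energy; Tick uses a Delay to count down the Q and R cooldowns.
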(event `self.ReceiveBeginPlay`
  (`parent.ReceiveBeginPlay`))

(event `ResetCanUseSkill`
  (set `self.bCanUseSkill1` true)
  (bind _gameplaywb (`/Game/FPS/Blueprints/PlayerController/BaseCharacterPC.GameplayWB` (`self.ControllerRef`))
    (:`then`
      (`/Game/FPS/WidgetBP/WB_Gameplay.Skill1Reset` _gameplaywb))
    (:`else`)))

(event `self.UseClassSkill1`
  ;[0.8079 1 0.4961] Class Skill
  (if (`self.bCanUseSkill1`)
    (set `self.bCanUseSkill1` false)
    (bind _returnvalue (`KismetSystemLibrary.K2_SetTimerDelegate` (delegate `ResetCanUseSkill`) (`self.AbilityCoolDown`)))
    (`/Game/FPS/WidgetBP/WB_Gameplay.OnSkill1Used` (stale `ResetCanUseSkill` _gameplaywb) _returnvalue)
    (`self.Server`)
    (`self.UpdateRun`)
    (`GameplayStatics.PlaySound2D` "/Engine/VREditor/Sounds/UI/Floating_UI_Open-001.Floating_UI_Open-001" 1.0 1.0 0.0 null null)
    (`KismetSystemLibrary.Delay` 2.0)
    (`self.ServerResetRun`)
    (`self.UpdateRun`)))

(event `Server`
  ;[0.8079 1 0.4961] Class Skill
  (set `self.RunSpeedModifier` 2.5))

(event `ServerResetRun`
  ;[0.8079 1 0.4961] Class Skill
  (set `self.RunSpeedModifier` (`self.DefaultRunSpeedModdifier`)))

(event `self.ReceiveTick`
  (params (DeltaSeconds :type "Float (single-precision)"))
  (`KismetSystemLibrary.Delay` 1.0)
  (set `self.CoolDown` (- (`self.CoolDown`) 1.0))
  (set `self.Skill1CoolDown` (- (`self.Skill1CoolDown`) 1)))

(event `Set Ultimate Energy`
  (params (Energy :type Integer))
  ;[1 1 1] Set Ultimate Energy
  (set `self.Ultimate Energy` Energy))

(event `SpawnSkill`
  ;[1 1 1] Server Ground Shield
  (if (== (`self.Skill1CoolDown`) 0)
    (`self.SpawnSkillAll`)))

(event `Key|Q`
  (params (Key :type "Key Structure"))
  ;[1 1 1] Create Ground Shield
  (:`Pressed`
    (`self.SpawnSkill`)))

(event `SpawnSkillAll`
  (bind _returnvalue (`KismetMathLibrary.MakeTransform` (`KismetMathLibrary.MakeVector` (.x (.location (`self.GetTransform` self))) (.y (.location (`self.GetTransform` self))) (- (.z (.location (`self.GetTransform` self))) 15.0)) (.rotation (`self.GetTransform` self)) (.scale (`self.GetTransform` self))))
  ;[1 1 1] Server Ground Shield
  (if (`self.ActorHasTag` self "TeamA")
    (`|SpawnActorFromClass` "/Game/FPS/Blueprints/Skills/Skill1.Skill1_C" _returnvalue "Undefined" "OverrideRootScale" null null)
    (else
      (`|SpawnActorFromClass` "/Game/FPS/Blueprints/Skills/Skill1B.Skill1B_C" _returnvalue "Undefined" "OverrideRootScale" null null))))

(event `Key|R`
  (params (Key :type "Key Structure"))
  ;[1 1 1] Skill3
  (:`Pressed`
    (if (and (>= (`self.Ultimate Energy`) (`self.EnergyCostPerCharge`)) (<= (`self.CoolDown`) 0.0))
      (set `self.CoolDown` 4.0)
      (set `self.Ultimate Energy` (- (`self.Ultimate Energy`) (`self.EnergyCostPerCharge`)))
      (`self.SpawnSkill3`))))

(event `SpawnSkill2`
  ;[1 1 1] Create Skill2
  (`self.SpawnSkill2All`))

(event `Key|F`
  (params (Key :type "Key Structure"))
  ;[1 1 1] Create Skill2
  (:`Pressed`
    (if (> (`self.RepelenishTime`) 0.0)
      (set `self.RepelenishTime` 5.0)
      (`self.SpawnSkill2`))))

(event `SpawnSkill2All`
  (bind _returnvalue (`KismetMathLibrary.MakeTransform` (+ (.location (`self.GetTransform`)) 5.0) (.rotation (`self.GetTransform`)) (.scale (`self.GetTransform`))))
  ;[1 1 1] Create Skill2
  (if (`self.ActorHasTag` self "TeamA")
    (`|SpawnActorFromClass` "/Game/FPS/Blueprints/Skills/Skill2.Skill2_C" _returnvalue "Undefined" "OverrideRootScale" null null)
    (else
      (`|SpawnActorFromClass` "/Game/FPS/Blueprints/Skills/Skill2B.Skill2B_C" _returnvalue "Undefined" "OverrideRootScale" null null))))

(event `SpawnSkill3`
  ;[1 1 1] Skill3
  (`self.Spawn Skill All 3`))

(event `Spawn Skill All 3`
  (bind _returnvalue (`KismetMathLibrary.MakeTransform` (+ (.location (`self.GetTransform`)) 5.0) (.rotation (`self.GetTransform`)) (.scale (`self.GetTransform`))))
  ;[1 1 1] Skill3
  (if (`self.ActorHasTag` self "TeamA")
    (`|SpawnActorFromClass` "/Game/FPS/Blueprints/Skills/Skill3.Skill3_C" _returnvalue "Undefined" "OverrideRootScale" null null)
    (else
      (`|SpawnActorFromClass` "/Game/FPS/Blueprints/Skills/Skill3B.Skill3B_C" _returnvalue "Undefined" "OverrideRootScale" null null))))

(fn `UserConstructionScript`
  (`parent.UserConstructionScript`))