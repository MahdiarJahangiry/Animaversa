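; Playable support class character with two cooldown skills and an ultimate, reporting to the gameplay HUD.
; Skill 1 server-spawns an actor attached to the capsule.
; Skill 2 equips a grenade, thrown with hold-timed force or placed below by Aim, then detonated on reuse or by a delayed RepNotify.
; The ultimate equips a launcher, marks opposing-team characters via camera traces, and fires missiles at them on Fire or countdown, then restores the rifle.
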(event `ResetSkill`
  ;[1 1 1] Reset Skill
  (set `self.bCanUseSkill1` true)
  (`/Game/FPS/WidgetBP/WB_Gameplay.Skill1Reset` (`/Game/FPS/Blueprints/PlayerController/BaseCharacterPC.GameplayWB` (`self.ControllerRef`))))

(event `self.UseClassSkill1`
  (bind _bcanuseskill1 (`self.bCanUseSkill1`))
  ;[0.6685 0.7443 1] Class Skill
  (`KismetSystemLibrary.PrintString` (`KismetStringLibrary.Conv_BoolToString` _bcanuseskill1))
  (if _bcanuseskill1
    (`KismetSystemLibrary.PrintString` "Skill 1 used")
    (set `self.bCanUseSkill1` false)
    (bind _returnvalue (`KismetSystemLibrary.K2_SetTimerDelegate` (delegate `ResetSkill`) (`self.AbilityCoolDown`)))
    (`/Game/FPS/WidgetBP/WB_Gameplay.OnSkill1Used` (`/Game/FPS/Blueprints/PlayerController/BaseCharacterPC.GameplayWB` (`self.ControllerRef`)) _returnvalue)
    (`GameplayStatics.PlaySound2D` "/Engine/VREditor/Sounds/UI/Object_PickUp.Object_PickUp" 1.0 1.0 0.0 null null)
    (`self.Server_spawn` (`KismetMathLibrary.Conv_VectorToTransform` (`self.K2_GetActorLocation`)))))

(event `Server_spawn`
  (params (NewParam :type "Transform Structure"))
  ;[0.6685 0.7443 1] Class Skill
  (`self.ServerSpawnMine` NewParam self))

(event `ServerSpawnMine`
  (params (NewParam :type "Transform Structure") (pawn :type "Pawn Object Reference"))
  ;[0.6685 0.7443 1] Class Skill
  (bind _returnvalue (`|SpawnActorFromClass` "/Game/FPS/Blueprints/Skills/BP_skill1.BP_skill1_C" NewParam "Undefined" "OverrideRootScale" pawn pawn))
  (set `/Game/FPS/Blueprints/Skills/BP_skill1.controller_instigator` (`self.GetController` pawn) _returnvalue)
  (`self.K2_AttachToComponent` _returnvalue (`self.CapsuleComponent`) "None" "SnapToTarget" "SnapToTarget" "SnapToTarget" true))

(event `ResetCanUseSkill`
  ;[0.8079 1 0.4961] Class Skill2
  (set `self.bCanUseSkill2` true)
  (bind _gameplaywb (`/Game/FPS/Blueprints/PlayerController/BaseCharacterPC.GameplayWB` (`self.ControllerRef`))
    (:`then`
      (`/Game/FPS/WidgetBP/WB_Gameplay.Skill2Reset` _gameplaywb))
    (:`else`)))

(event `self.UseClassSkill2`
  ;[0.8079 1 0.4961] Class Skill2
  (if (`self.bCanUseSkill2`)
    (if (`self.Skill2 planted?`)
      (`self.Detonate_Skill2`)
      (elif (`self.Skill2Equip`)
        (if (not (`self.Hold_process_start`))
          (set `self.Skill2Equip` false)
          (`self.Throw_fast_skill_2` 1.0))
        (else
          (`self.Skill2_equip`))))))

(event `Detonate_Skill2`
  ;[0.8079 1 0.4961] Class Skill2
  (`self.Detonate_server`)
  (set `self.bCanUseSkill2` false)
  (set `self.Skill2Equip` false)
  (bind _returnvalue (`KismetSystemLibrary.K2_SetTimerDelegate` (delegate `ResetCanUseSkill`) (`self.AbilityCoolDown`)))
  (`/Game/FPS/WidgetBP/WB_Gameplay.OnSkill2Used` (stale `ResetCanUseSkill` _gameplaywb) _returnvalue)
  (set `self.Skill2 planted?` false))

(event `Detonate_server`
  ;[0.8079 1 0.4961] Class Skill2
  (`/Game/FPS/Blueprints/Skills/BP_Grenade1.Detonate` (`self.Skill2_Object`)))

(event `Spawn_Skill2_Server`
  (params (SpawnTransform :type "Transform Structure") (PawnVelocity :type "Float (double-precision)") (Secondary_throw :type Boolean) (Speed_multiplier :type "Float (double-precision)") (ParentActor :type "Actor Object Reference"))
  ;[0.8079 1 0.4961] Class Skill2
  (bind _returnvalue (`|SpawnActorFromClass` "/Game/FPS/Blueprints/Skills/BP_Grenade1.BP_Grenade1_C" SpawnTransform "Undefined" "OverrideRootScale" self 5.0 PawnVelocity Speed_multiplier Secondary_throw self))
  (set `self.Skill2_Object` _returnvalue)
  (`self.ForceChange`))

(event `self.OnRep_Skill2 planted?`
  ;[0.8079 1 0.4961] Class Skill2
  (if (`self.Skill2 planted?`)
    (`KismetSystemLibrary.Delay` (`self.Time to self detonate`))
    (`self.Detonate_Skill2`)))

(event `Throw_fast_skill_2`
  (params (Force :type "Float (double-precision)"))
  (bind (_returnvalue_location _returnvalue_rotation) (`KismetMathLibrary.BreakTransform` (`self.GetTransform`)))
  ;[0.8079 1 0.4961] Class Skill2
  (set `self.Skill2 planted?` true)
  (`AnimInstance.Montage_JumpToSection` (`SkeletalMeshComponent.GetAnimInstance` (`self.MeshFP`)) "ThrowEnd" "/Game/FPS/Animations/FPP_Animations/Grenade/Throw_Grenade_Montage.Throw_Grenade_Montage")
  (`self.Spawn_Skill2_Server` (`KismetMathLibrary.MakeTransform` (+ _returnvalue_location (0.0 0.0 100.0) (* (`self.GetActorForwardVector`) 100.0)) _returnvalue_rotation) (`KismetMathLibrary.VSize` (`self.GetVelocity`)) false Force))

(event `Secondary_throw`
  (bind (_returnvalue_location _returnvalue_rotation) (`KismetMathLibrary.BreakTransform` (`self.GetTransform`)))
  (bind _returnvalue (+ _returnvalue_location (0.0 0.0 100.0) (* (`self.GetActorForwardVector`) 100.0)))
  ;[0.8079 1 0.4961] Class Skill2
  (if (and (`self.Skill2Equip`) (not (`self.Skill2 planted?`)))
    (bind _outhit (`KismetSystemLibrary.LineTraceSingle` _returnvalue (- _returnvalue (0.0 0.0 500.0)) "TraceTypeQuery1"))
    (`self.Spawn_Skill2_Server` (`KismetMathLibrary.MakeTransform` (`.Location` (`GameplayStatics.BreakHitResult` _outhit)) _returnvalue_rotation) (`KismetMathLibrary.VSize` (`self.GetVelocity`)) true 0.0 (`.HitActor` (`GameplayStatics.BreakHitResult` _outhit)))
    (set `self.Skill2 planted?` true)))

(event `InputAction|Aim` :overrideparent false
  (params (Key :type "Key Structure"))
  ;[0.8079 1 0.4961] Class Skill2
  (:`Pressed`
    (`self.Secondary_throw`)))

(event `InputAction|Fire` :consume false :overrideparent false
  (params (Key :type "Key Structure"))
  ;[0.8079 1 0.4961] Class Skill2
  (:`Pressed`
    (switch `/Game/FPS/Blueprints/Weapons/EquipedWeaponEnum` (`self.EquipedWeapon`)
      (:`NewEnumerator4`
        (if (not (`self.Skill2 planted?`))
          (set `self.Hold_process_start` true)
          (bind _returnvalue (`KismetSystemLibrary.K2_SetTimerDelegate` (delegate `Detonates`) (`self.Skill2_fast_detonate_time`)))
          (`/Game/FPS/WidgetBP/WB_Gameplay.skill2_force_timer` (`self.GameplayWB_Ref`) true (`self.Skill2_fast_detonate_time`) _returnvalue)
          (goto _label :!via `Open`)))))
  (:`Released`
    (switch `/Game/FPS/Blueprints/Weapons/EquipedWeaponEnum` (`self.EquipedWeapon`)
      (:`NewEnumerator4`
        (`/Engine/EditorBlueprintResources/StandardMacros.Gate` true :!label _label
          (:`Exit`
            (`self.Throw_fast_skill_2` (/ (`KismetSystemLibrary.K2_GetTimerElapsedTimeHandle` _returnvalue) (`self.Skill2_fast_detonate_time`)) :!label _label_2)
            (set `self.Hold_process_start` false)
            (`self.ForceChange`)
            (`KismetSystemLibrary.K2_ClearAndInvalidateTimerHandle` _returnvalue)
            (`/Game/FPS/WidgetBP/WB_Gameplay.skill2_force_timer` :`self` (`self.GameplayWB_Ref`))
            (goto _label :!via `Close`)))))))

(event `Detonates`
  ;[0.8079 1 0.4961] Class Skill2
  (goto _label_2))

(event `self.UseUltimate`
  ;[1 1 1] Ultimate Skill
  (`self.Equip Ultimate Skill`))

(event `self.ReceiveTick`
  (params (DeltaSeconds :type "Float (single-precision)"))
  (bind _returnvalue (`SceneComponent.K2_GetComponentLocation` (`self.Camera`)))
  ;[1 1 1] Ultimate Skill
  (if (`self.CanUseUltimateFire`)
    (if (`self.ShotDealyActivated`)
      (bind _result (`/Engine/EditorBlueprintResources/StandardMacros.DecrementFloat` (`self.ShotDelay`))
        (:`  `
          (if (<= _result 0.0)
            (`self.AutoShot`)
            (else
              (bind (_outhit _returnvalue_2) (`KismetSystemLibrary.LineTraceSingleForObjects` :`Start` _returnvalue :`End` (+ _returnvalue (* (`KismetMathLibrary.GetForwardVector` (`Controller.GetControlRotation` (`self.GetController`))) 1500.0)) :`ObjectTypes` (`self.Object Types`) :`bTraceComplex` true :`DrawDebugType` "ForOneFrame" :!label _label_3))
              (if _returnvalue_2
                (bind _asbp_base_character (cast `/Game/FPS/Blueprints/CharacterAndClasses/BP_BaseCharacter` (`.HitActor` (`GameplayStatics.BreakHitResult` _outhit))))
                (if (`self.ActorHasTag` _asbp_base_character "TeamA")
                  (if (`self.ActorHasTag` self "TeamB")
                    (`|ExecutionSequence` :!label _label_4
                      (:`then_0`
                        (if (> (`KismetArrayLibrary.Array_Length` (`self.MarkedCharacter`)) 0)
                          (bind _result_2 (`/Engine/EditorBlueprintResources/StandardMacros.DecrementFloat` (`self.AutoShotTimer`))
                            (:`  `
                              (`KismetSystemLibrary.PrintString` (`KismetStringLibrary.Conv_DoubleToString` _result_2))
                              (if (<= _result_2 0.0)
                                (`KismetSystemLibrary.PrintString` "AutoShot")
                                (`self.AutoShot`))))))
                      (:`then_1`
                        (if (not (`/Game/FPS/Blueprints/CharacterAndClasses/BP_BaseCharacter.Marked` _asbp_base_character))
                          (`Widget.SetVisibility` (`WidgetComponent.GetUserWidgetObject` (`/Game/FPS/Blueprints/CharacterAndClasses/BP_BaseCharacter.Marker Widget` _asbp_base_character)) "Visible")
                          (set `/Game/FPS/Blueprints/CharacterAndClasses/BP_BaseCharacter.Marked` true _asbp_base_character)
                          (`KismetArrayLibrary.Array_Add` (`self.MarkedCharacter`) _asbp_base_character)))))
                  (elif (`self.ActorHasTag` self "TeamA")
                    (goto _label_4))))))))
      (else
        (goto _label_3)))))

(event `Equip Ultimate Skill`
  ;[1 1 1] Ultimate Skill
  (set `self.CanUseUltimateFire` true)
  (set `self.EquipedWeapon` "NewEnumerator5")
  (set `self.CurrentWeapon` (`self.PrimaryWeapon`))
  (`self.PickUpWeapon` (`GameplayStatics.GetObjectClass` (`self.Lancher`)) 3))

(event `AutoShot`
  (bind _markedcharacter (`self.MarkedCharacter`))
  ;[1 1 1] Ultimate Skill
  (if (> (`KismetArrayLibrary.Array_Length` (`self.MarkedCharacter`)) 0) :!label _label_5
    (switch `/Game/FPS/Blueprints/Weapons/EquipedWeaponEnum` (`self.EquipedWeapon`)
      (:`NewEnumerator5`
        (for (_array_element _array_index) _markedcharacter :!label _label_6
          (set `self.CanTurn` false)
          (bind _output_get (set `self.Unmarked Ones` _array_element))
          (`self.CreateMissle` _output_get)
          (`KismetArrayLibrary.Array_Add` (`self.UnmarkedOnes`) _output_get)
          (`KismetArrayLibrary.Array_Remove` _markedcharacter _array_index))
        (set `self.bCanUseUltimate` false)
        (set `self.CanTurn` true)
        (`self.PickUpWeapon` "/Game/FPS/Blueprints/Weapons/BP_Rifle_Weapon.BP_Rifle_Weapon_C" 3)
        (set `self.AutoShotTimer` 100.0)
        (for _array_element_2 (`self.UnmarkedOnes`)
          (set `/Game/FPS/Blueprints/CharacterAndClasses/BP_BaseCharacter.Marked` false _array_element_2)
          (`Widget.SetVisibility` (`WidgetComponent.GetWidget` (`/Game/FPS/Blueprints/CharacterAndClasses/BP_BaseCharacter.Marker Widget` _array_element_2)) "Hidden"))))))

(event `InputAction|Fire` :consume false :overrideparent false
  (params (Key :type "Key Structure"))
  ;[1 1 1] Ultimate Skill
  (:`Pressed`
    (goto _label_5)))

(event `CreateMissle`
  (params (Character :type "/Game/FPS/Blueprints/CharacterAndClasses/BP_BaseCharacter Object Reference"))
  (bind _camera (`self.Camera`))
  (bind _returnvalue (`SceneComponent.K2_GetComponentLocation` _camera))
  ;[1 1 1] Ultimate Skill
  (set `self.OrgRotation` (`self.K2_GetActorRotation` self))
  (set `self.OrgLocation` _returnvalue)
  (`SceneComponent.K2_SetWorldTransform` _camera (`KismetMathLibrary.MakeTransform` _returnvalue (`KismetMathLibrary.FindLookAtRotation` (`self.K2_GetActorLocation` self) (`self.K2_GetActorLocation` Character))) false false)
  (`|SpawnActorFromClass` "/Game/FPS/Blueprints/Weapons/Missle.Missle_C" (`SceneComponent.K2_GetComponentToWorld` (`self.Camera`)) "Undefined" "OverrideRootScale" null null)
  (set `self.ShotDealyActivated` true)
  (set `self.ShotDelay` 100.0)
  (`self.Can Shot Again`))

(event `Can Shot Again`
  ;[1 1 1] Ultimate Skill
  (goto _label_6 :!via `Break`))

(event `Skill2_equip`
  ;[1 1 1] Skill2
  (`self.Unequip_weapon`)
  (set `self.Skill2Equip` true)
  (bind _output_get (set `self.EquipedWeapon` "NewEnumerator4"))
  (`self.SetWeaponEquiped` _output_get)
  (set `self.CurrentWeapon` null)
  (`|PlayMontage` (`self.MeshFP`) "/Game/FPS/Animations/FPP_Animations/Grenade/Grenade_Equip_Montage.Grenade_Equip_Montage"
    (:`OnBlendOut`
      (set `self.bChangingWeapon` false)
      (`self.Show_Grenade`))))

(fn `UserConstructionScript`
  (`parent.UserConstructionScript`))